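; Interactable button that selects the Gunner role and loads the Gunner level.
; On BeginPlay it binds the "gunner select" Socket.IO event, though no handler for it appears in the graph.
; Interacting emits "gunner select" to the server, fades the camera and audio out, then opens the level after a matching delay.
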(event `self.ReceiveBeginPlay`
  (`SocketIOClientComponent.BindEvent` (`self.SocketIOClient`) "gunner select" "/"))

(event `/Game/Blueprints/Interactable.Interact`
  (`KismetSystemLibrary.PrintString` "Selected the Gunner")
  (`SocketIOClientComponent.Emit` (`self.SocketIOClient`) "gunner select" (`SIOJsonValue.ConstructJsonValueString` "gunner select") "/")
  (`PlayerCameraManager.StartCameraFade` :`self` (`GameplayStatics.GetPlayerCameraManager` 0) :`ToAlpha` 1.0 :`Duration` 3.0 :`bShouldFadeAudio` true :`bHoldWhenFinished` true)
  (`KismetSystemLibrary.Delay` 3.0)
  (`GameplayStatics.OpenLevel` "Gunner"))

(fn `UserConstructionScript`)