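; Alarm light actor for a submarine game that shows remaining health through its color.
; After a short delay on BeginPlay, it connects over Socket.IO to the game instance's server IP and decrements health on each "health_down" event.
; Low health starts a timeline blending the light between an alarm color and its default: yellow as a warning, red with boosted intensity and reach when critical.
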(event `self.ReceiveBeginPlay`
  (bind _socketioclient (`self.SocketIOClient`))
  (bind _socketioclient_2 (`self.SocketIOClient`))
  (bind _output_get (set `self.Current Alarm Color` (struct :`R` 0.341542 :`G` 0.71 :`B` 0.473695 :`A` 1.0)))
  (`LightComponent.SetLightColor` (`self.Alarm Light`) _output_get true)
  (`KismetSystemLibrary.Delay` 2.5)
  (bind _assubmarine_game_instance (cast `/Game/Blueprints/SubmarineGameInstance` (`GameplayStatics.GetGameInstance`)))
  (bind _output_get_2 (set `SocketIOClientComponent.AddressAndPort` (`/Game/Blueprints/SubmarineGameInstance.Server IP` _assubmarine_game_instance) _socketioclient))
  (`SocketIOClientComponent.Connect` _socketioclient _output_get_2)
  (`SocketIOClientComponent.BindEvent` _socketioclient_2 "life" "/")
  (`SocketIOClientComponent.BindEvent` _socketioclient_2 "health_down" "/"))

(event `Play Alarm`
  (bind (_direction _alarm_light_curve) (`Timeline|Alarm Light Curve` :!label _label)
    (:`Update`
      (`LightComponent.SetLightColor` (`self.Alarm Light`) (`KismetMathLibrary.LinearColorLerp` (`self.Current Alarm Color`) (`self.Default Light Color`) _alarm_light_curve) true)
      (goto _label :!via `Reverse`))))

(event `Stop Alarm`
  (goto _label :!via `Stop`))

(event `Refresh`
  (bind _alarm_light (`self.Alarm Light`))
  (if (> (`self.Health Left`) 2) :!label _label_2
    (`self.Stop Alarm`)
    (elif (== (`self.Health Left`) 2)
      (set `self.Current Alarm Color` (struct :`R` 0.85 :`G` 0.838941 :`B` 0.1615 :`A` 1.0))
      (`self.Play Alarm`)
      (elif (<= (`self.Health Left`) 1)
        (set `self.Current Alarm Color` (struct :`R` 0.975 :`G` 0.051672 :`A` 1.0))
        (`LightComponent.SetIntensity` _alarm_light 100000.0)
        (`PointLightComponent.SetAttenuationRadius` _alarm_light 16384.0)
        (`PointLightComponent.SetSourceRadius` _alarm_light 39.0)
        (`self.Play Alarm`)))))

(event `self.SocketIOClient.On`
  (params (Event :type String) (MessageJson :type "SIOJsonValue Object Reference"))
  (if (`KismetStringLibrary.EqualEqual_StrStr` Event "health_down")
    (`/Engine/EditorBlueprintResources/StandardMacros.DecrementInt` (`self.Health Left`)
      (:`  `
        (goto _label_2)))))

(fn `UserConstructionScript`)