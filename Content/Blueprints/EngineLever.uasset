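; An engine lever actor for a submarine game that rotates while interacted with and reports its position to a server over Socket.IO.
; On BeginPlay it connects to the server IP stored in the submarine game instance and binds a "lever" event, with no handler shown.
; The two interact events run a looping timer that steps the clamped roll up or down, emitting "engine lever" each tick until interaction ends.
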(event `self.ReceiveBeginPlay`
  (bind _socketioclient (`self.SocketIOClient`))
  (bind _assubmarine_game_instance (cast `/Game/Blueprints/SubmarineGameInstance` (`GameplayStatics.GetGameInstance`)))
  (bind _output_get (set `SocketIOClientComponent.AddressAndPort` (`/Game/Blueprints/SubmarineGameInstance.Server IP` _assubmarine_game_instance) _socketioclient))
  (`SocketIOClientComponent.Connect` _socketioclient _output_get)
  (`SocketIOClientComponent.BindEvent` (`self.SocketIOClient`) "lever" "/"))

(event `/Game/Blueprints/Interactable.Interact One`
  (params (Character :type "/Game/Blueprints/SubmarineCharacter Object Reference"))
  (set `self.Rotating Up` true)
  (set `self.Rotating Down` false)
  (`KismetSystemLibrary.K2_SetTimer` null "Handle Rotation" 0.013888888 true))

(event `/Game/Blueprints/Interactable.Interact One End`
  (params (Character :type "/Game/Blueprints/SubmarineCharacter Object Reference"))
  (set `self.Rotating Up` false)
  (set `self.Rotating Down` false)
  (`KismetSystemLibrary.K2_ClearTimer` null "Handle Rotation"))

(event `/Game/Blueprints/Interactable.Interact Two`
  (params (Character :type "/Game/Blueprints/SubmarineCharacter Object Reference"))
  (set `self.Rotating Up` false)
  (set `self.Rotating Down` true)
  (`KismetSystemLibrary.K2_SetTimer` null "Handle Rotation" 0.013888888 true))

(event `/Game/Blueprints/Interactable.Interact Two End`
  (params (Character :type "/Game/Blueprints/SubmarineCharacter Object Reference"))
  (set `self.Rotating Up` false)
  (set `self.Rotating Down` false)
  (`KismetSystemLibrary.K2_ClearTimer` null "Handle Rotation"))

(event `Handle Rotation`
  (bind _rotation (`self.Rotation`))
  (bind _defaultsceneroot (`self.DefaultSceneRoot`))
  (`|ExecutionSequence`
    (:`then_0`
      (if (`self.Rotating Up`)
        (bind _result (`/Engine/EditorBlueprintResources/StandardMacros.IncrementInt` _rotation)
          (:`  `
            (if (>= _result 160)
              (set `self.Rotation` 160))
            (`SocketIOClientComponent.Emit` (`self.SocketIOClient`) "engine lever" (`SIOJsonValue.ConstructJsonValueNumber` (`KismetMathLibrary.Conv_IntToDouble` (`self.Rotation`))) "/")
            (`SceneComponent.K2_SetRelativeRotation` _defaultsceneroot (`KismetMathLibrary.MakeRotator` (`KismetMathLibrary.Conv_IntToDouble` (`self.Rotation`)) (.pitch (`SceneComponent.RelativeRotation` _defaultsceneroot)) (.yaw (`SceneComponent.RelativeRotation` _defaultsceneroot))) false false :!label _label)))))
    (:`then_1`
      (if (`self.Rotating Down`)
        (bind _result_2 (`/Engine/EditorBlueprintResources/StandardMacros.DecrementInt` _rotation)
          (:`  `
            (if (< _result_2 20)
              (set `self.Rotation` 20))
            (`SocketIOClientComponent.Emit` (`self.SocketIOClient`) "engine lever" (`SIOJsonValue.ConstructJsonValueNumber` (`KismetMathLibrary.Conv_IntToDouble` (`self.Rotation`))) "/")
            (goto _label)))))))

(fn `UserConstructionScript`)