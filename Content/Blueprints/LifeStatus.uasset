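; LifeStatus is an interactable display of remaining lives, using three point lights and a SocketIO client.
; Refresh colors each light green or red by comparing HealthLeft against thresholds of one, two and three.
; HealthDown decrements HealthLeft without refreshing the lights itself.
; BeginPlay binds the socket "life" event, and Interact prints the count and emits a "life" message.
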(event `self.ReceiveBeginPlay`
  (`SocketIOClientComponent.BindEvent` (`self.SocketIOClient`) "life" "/"))

(event `/Game/Blueprints/Interactable.Interact`
  (`KismetSystemLibrary.PrintString` (`KismetStringLibrary.Concat_StrStr` "You have " (`KismetStringLibrary.Conv_IntToString` (`self.HealthLeft`)) " lives left"))
  (`SocketIOClientComponent.Emit` (`self.SocketIOClient`) "life" (`SIOJsonValue.ConstructJsonValueString` "life") "/"))

(event `Refresh`
  (bind _pointlight1 (`self.PointLight1`))
  (bind _pointlight2 (`self.PointLight2`))
  (bind _pointlight (`self.PointLight`))
  (`/Engine/EditorBlueprintResources/StandardMacros.CompareInt` (`self.HealthLeft`) 1
    (:`>`
      (`LightComponent.SetLightColor` _pointlight (struct :`G` 1.0 :`A` 1.0) true :!label _label))
    (:`==`
      (goto _label))
    (:`<`
      (`LightComponent.SetLightColor` _pointlight (struct :`R` 1.0 :`A` 1.0) true)))
  (`/Engine/EditorBlueprintResources/StandardMacros.CompareInt` (`self.HealthLeft`) 2
    (:`>`
      (`LightComponent.SetLightColor` _pointlight1 (struct :`G` 1.0 :`A` 1.0) true :!label _label_2))
    (:`==`
      (goto _label_2))
    (:`<`
      (`LightComponent.SetLightColor` _pointlight1 (struct :`R` 1.0 :`A` 1.0) true)))
  (`/Engine/EditorBlueprintResources/StandardMacros.CompareInt` (`self.HealthLeft`) 3
    (:`>`
      (`LightComponent.SetLightColor` _pointlight2 (struct :`G` 1.0 :`A` 1.0) true :!label _label_3))
    (:`==`
      (goto _label_3))
    (:`<`
      (`LightComponent.SetLightColor` _pointlight2 (struct :`R` 1.0 :`A` 1.0) true))))

(event `Health Down`
  (set `self.HealthLeft` (- (`self.HealthLeft`) 1)))

(fn `UserConstructionScript`)