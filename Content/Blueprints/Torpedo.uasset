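; Torpedo actor that a character can pick up and carry, lock in place and launch.
; On BeginPlay or Colorize, actor tags choose the band material: red, green, or blue by default.
; Interaction sets the holder's held item and toggles physics, while locking clears the held item, straightens rotation and freezes physics.
; Launching rescales six P components and moves the torpedo upward by a fixed, frame-dependent step each Tick.
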(event `Colorize`
  (bind _band (`self.Band`))
  (bind _tags (`self.Tags`))
  (if (`KismetArrayLibrary.Array_Contains` _tags "Red") :!label _label
    (`PrimitiveComponent.SetMaterial` _band 0 "/Game/Assets/materials/05_-_Default.05_-_Default")
    (elif (`KismetArrayLibrary.Array_Contains` _tags "Green")
      (`PrimitiveComponent.SetMaterial` _band 0 "/Engine/EngineDebugMaterials/VertexColorViewMode_GreenOnly.VertexColorViewMode_GreenOnly")
      (else
        (`PrimitiveComponent.SetMaterial` _band 0 "/Engine/TemplateResources/MI_Template_BaseBlue.MI_Template_BaseBlue")))))

(event `self.ReceiveBeginPlay`
  (goto _label))

(event `/Game/Blueprints/Interactable.Interact One`
  (params (Character :type "/Game/VirtualRealityBP/Blueprints/MotionControllerPawn Object Reference"))
  (bind _root (`self.Root`))
  (set `/Game/VirtualRealityBP/Blueprints/MotionControllerPawn.Held Item` _root Character)
  (`PrimitiveComponent.SetSimulatePhysics` _root false)
  (set `self.Holding Character` Character))

(event `/Game/Blueprints/Interactable.Interact One End`
  (params (Character :type "/Game/VirtualRealityBP/Blueprints/MotionControllerPawn Object Reference"))
  (set `/Game/VirtualRealityBP/Blueprints/MotionControllerPawn.Held Item` null Character)
  (`PrimitiveComponent.SetSimulatePhysics` (`self.Root`) true))

(event `Lock Torpedo`
  (set `/Game/VirtualRealityBP/Blueprints/MotionControllerPawn.Held Item` null (`self.Holding Character`))
  (`SceneComponent.K2_SetWorldRotation` :`self` (`self.Root`))
  (`PrimitiveComponent.SetSimulatePhysics` (`self.Root`) false))

(event `self.ReceiveTick`
  (params (DeltaSeconds :type "Float (single-precision)"))
  (if (`self.Launching`)
    (`SceneComponent.K2_AddWorldTransform` (`self.Root`) (`KismetMathLibrary.MakeTransform` (0.0 0.0 5.0)) false false)))

(event `Launch Torpedo`
  (set `self.Launching` true)
  (`SceneComponent.SetWorldScale3D` (`self.P1`) (1.0 1.0 1.0))
  (`SceneComponent.SetWorldScale3D` (`self.P2`) (1.0 1.0 1.0))
  (`SceneComponent.SetWorldScale3D` (`self.P3`) (1.0 1.0 1.0))
  (`SceneComponent.SetWorldScale3D` (`self.P4`) (1.0 1.0 1.0))
  (`SceneComponent.SetWorldScale3D` (`self.P5`) (1.0 1.0 1.0))
  (`SceneComponent.SetWorldScale3D` (`self.P6`) (1.0 1.0 1.0)))

(fn `UserConstructionScript`)