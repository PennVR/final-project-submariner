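; ConnectionManager links the submarine game to a Socket.IO server and handles end-of-match results.
; After a short delay on BeginPlay, it connects to the server IP stored in SubmarineGameInstance and binds "win" and "lose" events.
; Either event prints the result, fades camera and audio (red for a loss), then opens the Lobby level.
; A separate DisconnectAll event disconnects and clears every entry in ActiveClients.
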(event `self.ReceiveBeginPlay`
  (bind _socketioclient (`self.SocketIOClient`))
  (`KismetSystemLibrary.Delay` 2.5)
  (bind _assubmarine_game_instance (cast `/Game/Blueprints/SubmarineGameInstance` (`GameplayStatics.GetGameInstance`)))
  (bind _output_get (set `SocketIOClientComponent.AddressAndPort` (`/Game/Blueprints/SubmarineGameInstance.Server IP` _assubmarine_game_instance) _socketioclient))
  (`SocketIOClientComponent.Connect` _socketioclient _output_get)
  (`SocketIOClientComponent.BindEvent` (`self.SocketIOClient`) "win" "/")
  (`SocketIOClientComponent.BindEvent` (`self.SocketIOClient`) "lose" "/"))

(event `Disconnect All`
  (for _array_element (`self.ActiveClients`)
    (`SocketIOClientComponent.Disconnect` _array_element))
  (`KismetArrayLibrary.Array_Clear` (`self.ActiveClients`)))

(event `self.SocketIOClient.On`
  (params (Event :type String) (MessageJson :type "SIOJsonValue Object Reference"))
  (`|ExecutionSequence`
    (:`then_0`
      (if (`KismetStringLibrary.EqualEqual_StrStr` Event "win")
        (`KismetSystemLibrary.PrintString` "!!! YOU WIN !!!")
        (`PlayerCameraManager.StartCameraFade` :`self` (`GameplayStatics.GetPlayerCameraManager` 0) :`ToAlpha` 1.0 :`Duration` 3.0 :`bShouldFadeAudio` true :`bHoldWhenFinished` true)
        (`KismetSystemLibrary.Delay` 3.0)
        (`GameplayStatics.OpenLevel` "Lobby")))
    (:`then_1`
      (if (`KismetStringLibrary.EqualEqual_StrStr` Event "lose")
        (`KismetSystemLibrary.PrintString` "!!! YOU LOSE !!!")
        (`PlayerCameraManager.StartCameraFade` (`GameplayStatics.GetPlayerCameraManager` 0) 0.0 1.0 3.0 (struct :`R` 1.0 :`A` 1.0) true true)
        (`KismetSystemLibrary.Delay` 3.0)
        (`GameplayStatics.OpenLevel` "Lobby")))))

(fn `UserConstructionScript`)