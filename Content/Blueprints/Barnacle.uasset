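; Barnacle hazard actor for the submarine game that reports a breach to a Socket.IO server if left in place too long.
; On BeginPlay it connects to the game instance's server IP and binds the "barnacle" event.
; SpawnBarnacle starts a looping one-second countdown, which emits the breach message at zero, then clears tags and destroys the actor.
; InteractTwo fires the character's M1 at the barnacle and removes it without reporting.
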(event `self.ReceiveBeginPlay`
  (bind _socketioclient (`self.SocketIOClient`))
  (bind _assubmarine_game_instance (cast `/Game/Blueprints/SubmarineGameInstance` (`GameplayStatics.GetGameInstance`)))
  (bind _output_get (set `SocketIOClientComponent.AddressAndPort` (`/Game/Blueprints/SubmarineGameInstance.Server IP` _assubmarine_game_instance) _socketioclient))
  (`SocketIOClientComponent.Connect` _socketioclient _output_get)
  (`SocketIOClientComponent.BindEvent` (`self.SocketIOClient`) "barnacle" "/"))

(event `Spawn Barnacle`
  (`KismetSystemLibrary.K2_SetTimerDelegate` (delegate `TimerDown`) 1.0 true))

(event `TimerDown`
  (bind _output_get (set `self.Timer` (- (`self.Timer`) 1)))
  (if (<= _output_get 0)
    (`SocketIOClientComponent.Emit` (`self.SocketIOClient`) "barnacle" (`SIOJsonValue.ConstructJsonValueString` "barnacle breach") "/")
    (`KismetArrayLibrary.Array_Clear` (`self.Tags`) :!label _label)
    (`self.K2_DestroyActor`)))

(event `/Game/Blueprints/Interactable.Interact Two`
  (params (Character :type "/Game/VirtualRealityBP/Blueprints/MotionControllerPawn Object Reference"))
  (`/Game/Blueprints/M1.Fire` (`/Game/VirtualRealityBP/Blueprints/MotionControllerPawn.M1` Character) (`SceneComponent.K2_GetComponentLocation` (`self.Barnacle`)))
  (goto _label))

(fn `UserConstructionScript`)