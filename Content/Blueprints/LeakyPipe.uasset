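; Leaky pipe hazard actor for a submarine game that counts down once spawned and reports to a server if it runs out.
; On BeginPlay it connects a SocketIO client to the game instance's server IP and binds the engine_pipe event.
; SpawnLeakyPipe starts a one-second looping timer that decrements Timer, emitting engine_pipe and destroying the actor at zero.
; Either interact event destroys the pipe without emitting.
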(event `self.ReceiveBeginPlay`
  (bind _socketioclient (`self.SocketIOClient`))
  (bind _assubmarine_game_instance (cast `/Game/Blueprints/SubmarineGameInstance` (`GameplayStatics.GetGameInstance`)))
  (bind _output_get (set `SocketIOClientComponent.AddressAndPort` (`/Game/Blueprints/SubmarineGameInstance.Server IP` _assubmarine_game_instance) _socketioclient))
  (`SocketIOClientComponent.Connect` _socketioclient _output_get)
  (`SocketIOClientComponent.BindEvent` (`self.SocketIOClient`) "engine_pipe" "/"))

(event `Spawn Leaky Pipe`
  (`KismetSystemLibrary.K2_SetTimerDelegate` (delegate `TimerDown`) 1.0 true))

(event `TimerDown`
  (bind _output_get (set `self.Timer` (- (`self.Timer`) 1)))
  (if (== _output_get 0)
    (`SocketIOClientComponent.Emit` (`self.SocketIOClient`) "engine_pipe" null "/")
    (`self.K2_DestroyActor` :!label _label)))

(event `/Game/Blueprints/Interactable.Interact One`
  (params (Character :type "/Game/Blueprints/SubmarineCharacter Object Reference"))
  (goto _label))

(event `/Game/Blueprints/Interactable.Interact Two`
  (params (Character :type "/Game/Blueprints/SubmarineCharacter Object Reference"))
  (goto _label))

(fn `UserConstructionScript`)