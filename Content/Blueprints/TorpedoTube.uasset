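; Torpedo tube actor that loads torpedoes pushed into its trigger box.
; On overlap, an actor tagged Red, Green or Blue that casts to Torpedo is stored as the loaded torpedo, snapped to the TorpedoLock position and locked.
; The loaded torpedo is then handed to the FiringHandle, with debug prints on overlap and load.
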(event `self.ReceiveBeginPlay`
  (add `PrimitiveComponent.OnComponentBeginOverlap` (`self.TriggerBox`) (delegate `Torpedo Overlaps`)))

(event `Torpedo Overlaps`
  (params (OverlappedComponent :type "PrimitiveComponent Object Reference") (OtherActor :type "Actor Object Reference") (OtherComp :type "PrimitiveComponent Object Reference") (OtherBodyIndex :type Integer) (bFromSweep :type Boolean) (SweepResult :type "HitResult Structure (by ref)"))
  (bind _tags (`Actor.Tags` OtherActor))
  (`KismetSystemLibrary.PrintString` "Overlap")
  (if (or (`KismetArrayLibrary.Array_Contains` _tags "Red") (`KismetArrayLibrary.Array_Contains` _tags "Green") (`KismetArrayLibrary.Array_Contains` _tags "Blue"))
    (bind _astorpedo (cast `/Game/Blueprints/Torpedo` OtherActor))
    (bind _output_get (set `self.Loaded Torpedo` _astorpedo))
    (`SceneComponent.K2_SetWorldLocation` (`/Game/Blueprints/Torpedo.Root` _output_get) (`SceneComponent.K2_GetComponentLocation` (`self.TorpedoLock`)) false false)
    (`/Game/Blueprints/Torpedo.Lock Torpedo` _output_get)
    (`KismetSystemLibrary.PrintString` "Torpedo Loaded")
    (set `/Game/Blueprints/GunnerHandle.Torpedo` (`self.Loaded Torpedo`) (`self.Firing Handle`))))

(fn `UserConstructionScript`)