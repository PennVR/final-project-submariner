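; Lobby connection actor that links the game to a Socket.IO server for crew role selection in the submarine game.
; On BeginPlay it waits briefly, reads the server IP from SubmarineGameInstance and connects its SocketIOClient component to that address.
; It then binds the captain, gunner, navigator and engineer select events on the root namespace, with no handlers for them in this graph.
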(event `self.ReceiveBeginPlay`
  (`KismetSystemLibrary.Delay` 2.5)
  (bind _assubmarine_game_instance (cast `/Game/Blueprints/SubmarineGameInstance` (`GameplayStatics.GetGameInstance`)))
  (set `self.Server IP` (`/Game/Blueprints/SubmarineGameInstance.Server IP` _assubmarine_game_instance))
  (bind _output_get (set `SocketIOClientComponent.AddressAndPort` (`self.Server IP`) (`self.SocketIOClient`)))
  (`SocketIOClientComponent.Connect` (`self.SocketIOClient`) _output_get null null)
  (`SocketIOClientComponent.BindEvent` (`self.SocketIOClient`) "captain select" "/")
  (`SocketIOClientComponent.BindEvent` (`self.SocketIOClient`) "gunner select" "/")
  (`SocketIOClientComponent.BindEvent` (`self.SocketIOClient`) "navigator select" "/")
  (`SocketIOClientComponent.BindEvent` (`self.SocketIOClient`) "engineer select" "/"))

(fn `UserConstructionScript`)