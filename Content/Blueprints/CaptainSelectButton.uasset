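; An interactable button that lets a player pick the Captain role in a networked submarine game.
; On BeginPlay it connects its SocketIO client to the server IP stored in the SubmarineGameInstance and binds the "captain select" event, with no handler shown.
; On interaction it emits that event, fades the camera and audio out, then opens the Captain level once the fade completes.
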(event `self.ReceiveBeginPlay`
  (bind _socketioclient (`self.SocketIOClient`))
  (bind _assubmarine_game_instance (cast `/Game/Blueprints/SubmarineGameInstance` (`GameplayStatics.GetGameInstance`)))
  (bind _output_get (set `SocketIOClientComponent.AddressAndPort` (`/Game/Blueprints/SubmarineGameInstance.Server IP` _assubmarine_game_instance) _socketioclient))
  (`SocketIOClientComponent.Connect` _socketioclient _output_get)
  (`SocketIOClientComponent.BindEvent` _socketioclient "captain select" "/"))

(event `/Game/Blueprints/Interactable.Interact One`
  (`KismetSystemLibrary.PrintString` "Selected the Captain")
  (`SocketIOClientComponent.Emit` (`self.SocketIOClient`) "captain select" (`SIOJsonValue.ConstructJsonValueString` "captain select") "/")
  (`PlayerCameraManager.StartCameraFade` :`self` (`GameplayStatics.GetPlayerCameraManager` 0) :`ToAlpha` 1.0 :`Duration` 3.0 :`bShouldFadeAudio` true :`bHoldWhenFinished` true)
  (`KismetSystemLibrary.Delay` 3.0)
  (`GameplayStatics.OpenLevel` "Captain"))

(fn `UserConstructionScript`)