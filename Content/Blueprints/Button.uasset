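; Button is an interactable actor that notifies a Socket.IO server when the player interacts with it.
; On BeginPlay it takes the server address from SubmarineGameInstance, connects its SocketIOClient component and binds the "button" event.
; InteractOne prints a debug string and emits a "button" message on the root namespace.
; No handler for the bound incoming event appears in the graph.
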(event `self.ReceiveBeginPlay`
  (bind _socketioclient (`self.SocketIOClient`))
  (bind _assubmarine_game_instance (cast `/Game/Blueprints/SubmarineGameInstance` (`GameplayStatics.GetGameInstance`)))
  (bind _output_get (set `SocketIOClientComponent.AddressAndPort` (`/Game/Blueprints/SubmarineGameInstance.Server IP` _assubmarine_game_instance) _socketioclient))
  (`SocketIOClientComponent.Connect` _socketioclient _output_get)
  (`SocketIOClientComponent.BindEvent` _socketioclient "button" "/"))

(event `/Game/Blueprints/Interactable.Interact One`
  (`KismetSystemLibrary.PrintString` "I am a button")
  (`SocketIOClientComponent.Emit` (`self.SocketIOClient`) "button" (`SIOJsonValue.ConstructJsonValueString` "button") "/"))

(fn `UserConstructionScript`)