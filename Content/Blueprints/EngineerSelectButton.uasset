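; Interactable button Blueprint that selects the Engineer and loads the Engineer level.
; On BeginPlay it binds the "engineer select" event on its SocketIO client, with no handler for received messages in the graph.
; Interacting prints a debug message, emits that event to the server, fades the camera and audio out, then opens the level once the delay matching the fade ends.
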(event `self.ReceiveBeginPlay`
  (`SocketIOClientComponent.BindEvent` (`self.SocketIOClient`) "engineer select" "/"))

(event `/Game/Blueprints/Interactable.Interact`
  (`KismetSystemLibrary.PrintString` "Selected the Engineer")
  (`SocketIOClientComponent.Emit` (`self.SocketIOClient`) "engineer select" (`SIOJsonValue.ConstructJsonValueString` "engineer select") "/")
  (`PlayerCameraManager.StartCameraFade` :`self` (`GameplayStatics.GetPlayerCameraManager` 0) :`ToAlpha` 1.0 :`Duration` 3.0 :`bShouldFadeAudio` true :`bHoldWhenFinished` true)
  (`KismetSystemLibrary.Delay` 3.0)
  (`GameplayStatics.OpenLevel` "Engineer"))

(fn `UserConstructionScript`)