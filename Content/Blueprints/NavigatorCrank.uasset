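; Navigator crank for a submarine game that turns left or right while one of two interactions is held.
; Each interaction starts a looping timer that steps an integer yaw one degree per tick, wrapping around a full circle, and rotates the root component.
; Every step emits the angle over Socket.IO to the server IP from the game instance.
; The matching socket event is bound, but no handler appears here.
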(event `self.ReceiveBeginPlay`
  (bind _socketioclient (`self.SocketIOClient`))
  (bind _assubmarine_game_instance (cast `/Game/Blueprints/SubmarineGameInstance` (`GameplayStatics.GetGameInstance`)))
  (bind _output_get (set `SocketIOClientComponent.AddressAndPort` (`/Game/Blueprints/SubmarineGameInstance.Server IP` _assubmarine_game_instance) _socketioclient))
  (`SocketIOClientComponent.Connect` _socketioclient _output_get)
  (`SocketIOClientComponent.BindEvent` (`self.SocketIOClient`) "navigator crank" "/"))

(event `/Game/Blueprints/Interactable.Interact One`
  (set `self.RotatingLeft` true)
  (set `self.RotatingRight` false)
  (`KismetSystemLibrary.K2_SetTimer` null "Handle Rotation" 0.013888888 true))

(event `/Game/Blueprints/Interactable.Interact One End`
  (set `self.RotatingLeft` false)
  (set `self.RotatingRight` false)
  (`KismetSystemLibrary.K2_ClearTimer` null "Handle Rotation"))

(event `/Game/Blueprints/Interactable.Interact Two`
  (set `self.RotatingRight` true)
  (set `self.RotatingLeft` false)
  (`KismetSystemLibrary.K2_SetTimer` null "Handle Rotation" 0.013888888 true))

(event `/Game/Blueprints/Interactable.Interact Two End`
  (set `self.RotatingRight` false)
  (set `self.RotatingLeft` false)
  (`KismetSystemLibrary.K2_ClearTimer` null "Handle Rotation"))

(event `Handle Rotation`
  (bind _rotation (`self.Rotation`))
  (bind _root (`self.Root`))
  (`|ExecutionSequence`
    (:`then_0`
      (if (`self.RotatingLeft`)
        (bind _result (`/Engine/EditorBlueprintResources/StandardMacros.IncrementInt` _rotation)
          (:`  `
            (if (>= _result 360)
              (set `self.Rotation` 0))
            (`SocketIOClientComponent.Emit` (`self.SocketIOClient`) "navigator crank" (`SIOJsonValue.ConstructJsonValueNumber` (`KismetMathLibrary.Conv_IntToDouble` (`self.Rotation`))) "/")
            (`SceneComponent.K2_SetRelativeRotation` _root (`KismetMathLibrary.MakeRotator` (.roll (`SceneComponent.RelativeRotation` _root)) (.pitch (`SceneComponent.RelativeRotation` _root)) (`KismetMathLibrary.Conv_IntToDouble` (`self.Rotation`))) false false :!label _label)))))
    (:`then_1`
      (if (`self.RotatingRight`)
        (bind _result_2 (`/Engine/EditorBlueprintResources/StandardMacros.DecrementInt` _rotation)
          (:`  `
            (if (< _result_2 0)
              (set `self.Rotation` 359))
            (`SocketIOClientComponent.Emit` (`self.SocketIOClient`) "navigator crank" (`SIOJsonValue.ConstructJsonValueNumber` (`KismetMathLibrary.Conv_IntToDouble` (`self.Rotation`))) "/")
            (goto _label)))))))

(fn `UserConstructionScript`)