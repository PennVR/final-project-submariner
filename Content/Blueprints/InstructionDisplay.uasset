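; InstructionDisplay is a Blueprint that shows instructions received from a Socket.IO server on a text render component in the submarine game.
; On BeginPlay it connects its SocketIO client to the server IP stored in SubmarineGameInstance and binds the "instruction" event.
; Each incoming message is saved to Instructions, set as the displayed text and printed for debugging.
; The construction script also renders the current Instructions value.
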(event `self.ReceiveBeginPlay`
  (bind _socketioclient (`self.SocketIOClient`))
  (bind _assubmarine_game_instance (cast `/Game/Blueprints/SubmarineGameInstance` (`GameplayStatics.GetGameInstance`)))
  (bind _output_get (set `SocketIOClientComponent.AddressAndPort` (`/Game/Blueprints/SubmarineGameInstance.Server IP` _assubmarine_game_instance) _socketioclient))
  (`SocketIOClientComponent.Connect` _socketioclient _output_get)
  (`SocketIOClientComponent.BindEvent` _socketioclient "instruction" "/"))

(event `self.SocketIOClient.On`
  (params (Event :type String) (MessageJson :type "SIOJsonValue Object Reference"))
  (bind _returnvalue (`SIOJsonValue.AsString` MessageJson))
  (if (`KismetStringLibrary.EqualEqual_StrStr` Event "instruction")
    (`KismetSystemLibrary.PrintString` _returnvalue)
    (set `self.Instructions` _returnvalue)
    (`TextRenderComponent.K2_SetText` (`self.TextRender`) (`KismetTextLibrary.Conv_StringToText` _returnvalue))
    (`KismetSystemLibrary.PrintString` _returnvalue)))

(fn `UserConstructionScript`
  (`TextRenderComponent.K2_SetText` (`self.TextRender`) (`KismetTextLibrary.Conv_StringToText` (`self.Instructions`))))