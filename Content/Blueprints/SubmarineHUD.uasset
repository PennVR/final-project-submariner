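; SubmarineHUD is a HUD Blueprint that draws a crosshair at the center of the screen.
; On each DrawHUD event, if the DrawHUD flag is true, it draws the Crosshair texture at a fixed square size.
; The position is half the screen size minus half the texture size, keeping the reticle centered at any resolution.
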(event `self.ReceiveDrawHUD`
  (params (SizeX :type Integer) (SizeY :type Integer))
  (bind _returnvalue (/ 32.0 2.0))
  (if (`self.DrawHUD`)
    (`self.DrawTexture` "/Game/Textures/crosshair.crosshair" (- (`KismetMathLibrary.Conv_IntToDouble` (/ SizeX 2)) _returnvalue) (- (`KismetMathLibrary.Conv_IntToDouble` (/ SizeY 2)) _returnvalue) 32.0 32.0 0.0 0.0 1.0 1.0)))

(fn `UserConstructionScript`)