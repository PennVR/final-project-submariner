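; TorpedoSpawner creates color-coded Torpedo actors through its SpawnTorpedo event.
; Each torpedo spawns at the TorpedoSpawn location with zero rotation and has physics simulation enabled on its root.
; The current color from TorpedoSelector is added to the torpedo as an actor tag, then Colorize is called on it.
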(event `Spawn Torpedo`
  (bind _returnvalue (`|SpawnActorFromClass` "/Game/Blueprints/Torpedo.Torpedo_C" (`KismetMathLibrary.MakeTransform` (`SceneComponent.K2_GetComponentLocation` (`self.TorpedoSpawn`))) "Undefined" "OverrideRootScale"))
  (`PrimitiveComponent.SetSimulatePhysics` (`/Game/Blueprints/Torpedo.Root` _returnvalue) true)
  (bind _tags (`Actor.Tags` _returnvalue))
  (`KismetArrayLibrary.Array_Add` _tags (`KismetStringLibrary.Conv_StringToName` (`/Game/Blueprints/TorpedoSelector.CurrentColor` (`self.TorpedoSelector`))))
  (set `Actor.Tags` _tags _returnvalue)
  (`/Game/Blueprints/Torpedo.Colorize` _returnvalue))

(fn `UserConstructionScript`)