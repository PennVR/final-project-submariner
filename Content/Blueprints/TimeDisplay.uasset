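; Countdown display actor that shows the match time limit received from a server as in-world text.
; On BeginPlay it connects a SocketIO client to the server IP stored in SubmarineGameInstance and binds the time_limit event.
; That event scales the received number down, writes it to the TextRender and starts a looping one-second Decrement timer.
; Decrement updates and debug-prints the value, clearing the timer once time runs out.
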(event `self.ReceiveBeginPlay`
  (bind _socketioclient (`self.SocketIOClient`))
  (bind _assubmarine_game_instance (cast `/Game/Blueprints/SubmarineGameInstance` (`GameplayStatics.GetGameInstance`)))
  (bind _output_get (set `SocketIOClientComponent.AddressAndPort` (`/Game/Blueprints/SubmarineGameInstance.Server IP` _assubmarine_game_instance) _socketioclient))
  (`SocketIOClientComponent.Connect` _socketioclient _output_get)
  (`SocketIOClientComponent.BindEvent` _socketioclient "time_limit" "/"))

(event `self.SocketIOClient.On`
  (params (Event :type String) (MessageJson :type "SIOJsonValue Object Reference"))
  (bind _returnvalue (/ (`KismetMathLibrary.Round` (`SIOJsonValue.AsNumber` MessageJson)) 10))
  (bind _returnvalue_2 (`KismetStringLibrary.Conv_IntToString` _returnvalue))
  (if (`KismetStringLibrary.EqualEqual_StrStr` Event "time_limit")
    (set `self.Time` _returnvalue)
    (`KismetSystemLibrary.PrintString` _returnvalue_2)
    (set `self.Time Display` _returnvalue_2)
    (`TextRenderComponent.K2_SetText` (`self.TextRender`) (`KismetTextLibrary.Conv_StringToText` _returnvalue_2))
    (`KismetSystemLibrary.K2_SetTimer` null "Decrement" 1.0 true)))

(event `Decrement`
  (bind _result (`/Engine/EditorBlueprintResources/StandardMacros.DecrementInt` (`self.Time`))
    (:`  `
      (bind _returnvalue (`KismetStringLibrary.Conv_IntToString` _result))
      (`KismetSystemLibrary.PrintString` _returnvalue)
      (set `self.Time Display` _returnvalue)
      (`TextRenderComponent.K2_SetText` (`self.TextRender`) (`KismetTextLibrary.Conv_StringToText` _returnvalue))
      (if (<= (`self.Time`) 0)
        (`KismetSystemLibrary.K2_ClearTimer` null "Decrement")))))

(fn `UserConstructionScript`
  (`TextRenderComponent.K2_SetText` (`self.TextRender`) (`KismetTextLibrary.Conv_StringToText` (`self.Time Display`))))